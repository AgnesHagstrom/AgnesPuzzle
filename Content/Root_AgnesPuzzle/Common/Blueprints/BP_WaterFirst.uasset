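; BP_WaterFirst is a puzzle water actor whose Water component moves between two positions when its TriggerBox is hit.
; BeginPlay stores the water's relative location as StartPos, and a timeline lerps it toward EndPos.
; Each hit plays or reverses the timeline depending on IfWatherISUp, a flag this graph reads but never sets.
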(event `self.ReceiveBeginPlay`
  (set `self.StartPos` (`SceneComponent.RelativeLocation` (`self.Water`))))

(event `self.TriggerBox.OnComponentHit`
  (params (HitComponent :type "PrimitiveComponent Object Reference") (OtherActor :type "Actor Object Reference") (OtherComp :type "PrimitiveComponent Object Reference") (NormalImpulse :type "Vector Structure") (Hit :type "HitResult Structure (by ref)"))
  (if (`self.bIfWatherISUp`)
    (bind (_direction _watherrising) (`Timeline|Timeline_0` :!via `Reverse` :!label _label)
      (:`Update`
        (`SceneComponent.K2_SetRelativeLocation` (`self.Water`) (`KismetMathLibrary.VLerp` (`self.StartPos`) (`self.EndPos`) _watherrising) false false)))
    (else
      (goto _label))))

(fn `UserConstructionScript`)