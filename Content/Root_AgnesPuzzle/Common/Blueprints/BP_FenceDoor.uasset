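; BP_FenceDoor is a puzzle gate and bridge that activates when a BP_Projectile hits its Trigger component.
; The hit plays a timeline that slides SMBridge between stored start and end positions.
; A one-second Delay on that timeline's update starts the Gate timeline, so the door begins rotating 90 degrees shortly after the bridge starts moving.
; Nothing in the graph reverses either motion.
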(event `self.Trigger.OnComponentHit`
  (params (HitComponent :type "PrimitiveComponent Object Reference") (OtherActor :type "Actor Object Reference") (OtherComp :type "PrimitiveComponent Object Reference") (NormalImpulse :type "Vector Structure") (Hit :type "HitResult Structure (by ref)"))
  (cast `/Game/Root_AgnesPuzzle/Core/Framework/BP_Projectile` OtherActor)
  (bind (_direction _bridge) (`Timeline|Timeline_0`)
    (:`Update`
      (`SceneComponent.K2_SetRelativeLocationAndRotation` :`self` (`self.SM_Bridge`) :`NewLocation` (`KismetMathLibrary.VLerp` (`self.StartPosBridge`) (`self.EndPosBridge`) _bridge))
      (`KismetSystemLibrary.Delay` 1.0)
      (bind (_direction_2 _newtrack_0) (`Timeline|Gate`)
        (:`Update`
          (`SceneComponent.K2_SetRelativeLocationAndRotation` (`self.Door`) (0.0 0.0 0.0) (`KismetMathLibrary.RLerp` (struct) (struct :`Yaw` 90.0) _newtrack_0) false false))))))

(fn `UserConstructionScript`)