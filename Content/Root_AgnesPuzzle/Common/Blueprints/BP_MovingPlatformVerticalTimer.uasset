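; BP_MovingPlatformVerticalTimer is a puzzle platform that moves its Door component when its Trigger is hit or when water rises.
; A hit runs a sped-up timeline that lerps between StartPos and EndPos, playing or reversing based on IsPlatformDown, which toggles on finish.
; MoveWithWater runs a slow second timeline if the platform is down, lerping from the Door's live Z toward an offset below WaterEndPos.
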(event `self.Trigger.OnComponentHit`
  (params (HitComponent :type "PrimitiveComponent Object Reference") (OtherActor :type "Actor Object Reference") (OtherComp :type "PrimitiveComponent Object Reference") (NormalImpulse :type "Vector Structure") (Hit :type "HitResult Structure (by ref)"))
  (`TimelineComponent.SetPlayRate` (`self.Timeline_0`) 3.0)
  (if (`self.bIsPlatformDown`)
    (bind (_direction _newtrack_0) (`Timeline|Timeline_0` :!via `Reverse` :!label _label)
      (:`Update`
        (`SceneComponent.K2_SetRelativeLocationAndRotation` :`self` (`self.Door`) :`NewLocation` (`KismetMathLibrary.VLerp` (`self.StartPos`) (`self.EndPos`) _newtrack_0)))
      (:`Finished`
        (if (`self.bIsPlatformDown`)
          (set `self.bIsPlatformDown` false)
          (else
            (set `self.bIsPlatformDown` true)))))
    (else
      (goto _label))))

(event `MoveWithWater`
  (params (ShouldRise :type Boolean) (WaterEndPos :type "Vector Structure"))
  (if ShouldRise
    (`TimelineComponent.SetPlayRate` (`self.Timeline_1`) 0.07)
    (if (`self.bIsPlatformDown`)
      (bind (_direction _newtrack_0) (`Timeline|Timeline_1`)
        (:`Update`
          (`SceneComponent.K2_SetRelativeLocationAndRotation` :`self` (`self.Door`) :`NewLocation` (`KismetMathLibrary.VLerp` (`KismetMathLibrary.MakeVector` 0.0 0.0 (.z (`SceneComponent.RelativeLocation` (`self.Door`)))) (`KismetMathLibrary.MakeVector` 0.0 0.0 (- (.z WaterEndPos) 200.0)) _newtrack_0)))
        (:`Finished`
          (if (`self.bIsPlatformDown`)
            (set `self.bIsPlatformDown` false)
            (else
              (set `self.bIsPlatformDown` true))))))))

(fn `UserConstructionScript`)