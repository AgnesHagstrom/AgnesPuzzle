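; BP_TriggerPhysics is a puzzle actor whose small box starts simulating physics when a projectile hits its trigger.
; The Trigger's hit event casts the other actor to BP_Projectile and, on success, enables physics on SmallBox.
; The construction script gives SmallBox a dynamic grey material instance, but the random color change that would use it is disconnected and never runs.
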(event `self.Trigger.OnComponentHit`
  (params (HitComponent :type "PrimitiveComponent Object Reference") (OtherActor :type "Actor Object Reference") (OtherComp :type "PrimitiveComponent Object Reference") (NormalImpulse :type "Vector Structure") (Hit :type "HitResult Structure (by ref)"))
  ;[1 1 1] Physics on the static mesh
  (cast `/Game/Root_AgnesPuzzle/Core/Framework/BP_Projectile` OtherActor)
  (`PrimitiveComponent.SetSimulatePhysics` (`self.SmallBox`) true))

(fn `UserConstructionScript`
  ;[1 1 1] Chreating the material that the that static mesh have
  (bind _returnvalue (`PrimitiveComponent.CreateDynamicMaterialInstance` (`self.SmallBox`) 0 "/Game/Root_AgnesPuzzle/Common/Environments/Materials/MI_Color_GreyLight.MI_Color_GreyLight" "None"))
  (set `self.Dynamic Material` _returnvalue))