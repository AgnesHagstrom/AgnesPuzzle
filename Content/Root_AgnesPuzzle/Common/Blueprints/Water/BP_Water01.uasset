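; BP_Water01 is a water gate Blueprint that moves a gate and raises or lowers water when its Box component is hit.
; The hit plays a timeline that lerps the gate between start and end positions, with its Update also feeding a Delay.
; After the delay, IsWaterUp selects playing or reversing a second timeline that lerps the water height, and that timeline toggles the flag when finished.
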(event `self.Box.OnComponentHit`
  (params (HitComponent :type "PrimitiveComponent Object Reference") (OtherActor :type "Actor Object Reference") (OtherComp :type "PrimitiveComponent Object Reference") (NormalImpulse :type "Vector Structure") (Hit :type "HitResult Structure (by ref)"))
  (bind (_direction _newtrack_0) (`Timeline|Watergat`)
    (:`Update`
      (`SceneComponent.K2_SetRelativeLocationAndRotation` :`self` (`self.WaterGate`) :`NewLocation` (`KismetMathLibrary.VLerp` (`self.StartPosGate`) (`self.EndPosGate`) _newtrack_0))
      (`KismetSystemLibrary.Delay` 4.5)
      (if (`self.bIsWaterUp`)
        (bind (_direction_2 _newtrack_0_2) (`Timeline|WaterRising` :!via `Reverse` :!label _label)
          (:`Update`
            (`SceneComponent.K2_SetRelativeLocation` (`self.Water`) (`KismetMathLibrary.VLerp` (`self.StarPosWater`) (`self.EndPosWater`) _newtrack_0_2) false false))
          (:`Finished`
            (if (`self.bIsWaterUp`)
              (set `self.bIsWaterUp` false)
              (else
                (set `self.bIsWaterUp` true)))))
        (else
          (goto _label))))))

(fn `UserConstructionScript`)