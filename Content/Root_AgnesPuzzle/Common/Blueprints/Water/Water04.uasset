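; Puzzle water body that alternates between two levels whenever its Trigger component registers a hit.
; The Water timeline plays or reverses based on IsWaterUp, lerping the SMWater mesh between start and end positions.
; Each timeline update calls MoveWithWater on every entry in Platforms, passing the current flag and the water's end position.
; IsWaterUp flips only when the timeline finishes, so it holds the pre-move state during travel.
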(event `self.Trigger.OnComponentHit`
  (params (HitComponent :type "PrimitiveComponent Object Reference") (OtherActor :type "Actor Object Reference") (OtherComp :type "PrimitiveComponent Object Reference") (NormalImpulse :type "Vector Structure") (Hit :type "HitResult Structure (by ref)"))
  (if (`self.bIsWaterUp`)
    (bind (_direction _newtrack_0) (`Timeline|Water` :!via `Reverse` :!label _label)
      (:`Update`
        (`SceneComponent.K2_SetRelativeLocationAndRotation` :`self` (`self.SM_Water`) :`NewLocation` (`KismetMathLibrary.VLerp` (`self.StartPosWater`) (`self.EndPosWater`) _newtrack_0))
        (for _array_element (`self.platforms`)
          (`/Game/Root_AgnesPuzzle/Common/Blueprints/BP_MovingPlatformVerticalTimer.MoveWithWater` _array_element (`self.bIsWaterUp`) (`self.EndPosWater`))))
      (:`Finished`
        (if (`self.bIsWaterUp`)
          (set `self.bIsWaterUp` false)
          (else
            (set `self.bIsWaterUp` true)))))
    (else
      (goto _label))))

(fn `UserConstructionScript`)