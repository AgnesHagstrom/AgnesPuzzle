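; Door trigger Blueprint for the Agnes puzzle that responds to a physics Hit event by starting a door timeline.
; The Hit passes through an always-true branch and a DoOnce gate before playing TimelineDoor.
; The door movement is unfinished: the position lerp and the Door transform call are disconnected, so the timeline moves nothing here.
; A random material color change is also left unconnected.
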(event `self.ReceiveHit`
  (params (MyComp :type "PrimitiveComponent Object Reference") (Other :type "Actor Object Reference") (OtherComp :type "PrimitiveComponent Object Reference") (bSelfMoved :type Boolean) (HitLocation :type "Vector Structure") (HitNormal :type "Vector Structure") (NormalImpulse :type "Vector Structure") (Hit :type "HitResult Structure (by ref)"))
  ;[1 1 1] Physics on the static mesh
  (if true
    (`/Engine/EditorBlueprintResources/StandardMacros.DoOnce` true
      (:`Completed`
        (bind (_direction _newtrack_0) (`Timeline|TimelineDoor` :`NewTime` 4.0))))))

(fn `UserConstructionScript`)