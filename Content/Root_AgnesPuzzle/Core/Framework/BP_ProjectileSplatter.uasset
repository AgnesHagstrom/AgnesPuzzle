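; BP_ProjectileSplatter is an impact splatter decal actor, spawned where a projectile leaves its mark.
; The construction script creates a dynamic material instance on the decal component.
; On BeginPlay it picks one of four texture variants through the Frame parameter and gives the decal a random roll for visual variety.
; It also spawns an ice impact particle effect at its location.
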(event `self.ReceiveBeginPlay`
  (`MaterialInstanceDynamic.SetScalarParameterValue` (`self.DynamicMaterial`) "Frame" (`KismetMathLibrary.Conv_IntToDouble` (`KismetMathLibrary.RandomIntegerInRange` 0 3))) ; Det finns 4a versioner av dekalen i samma \ntextur. Denna tar en random.
  (`SceneComponent.K2_SetRelativeRotation` (`self.Decal`) (`KismetMathLibrary.MakeRotator` (`KismetMathLibrary.RandomFloatInRange` 0.0 360.0)) false false) ; Sätter en random rotation
  (`GameplayStatics.SpawnEmitterAtLocation` "/Game/Root_AgnesPuzzle/Core/PlayerCharacter/FPWeapon/Effects/FX_Mobile/Impacts/P_Impact_Enemy_Ice_Medium.P_Impact_Enemy_Ice_Medium" (`self.K2_GetActorLocation`)))

(fn `UserConstructionScript`
  (bind _returnvalue (`DecalComponent.CreateDynamicMaterialInstance` (`self.Decal`)))
  (set `self.DynamicMaterial` _returnvalue))